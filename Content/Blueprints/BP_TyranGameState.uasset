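; BP_TyranGameState is a game state that ends the match after a fixed two-minute duration.
; BeginPlay stores the duration in seconds.
; Tick compares server world time against it and, once exceeded, calls the FinDuJeu event dispatcher a single time, guarded by the JeuFini flag.
; The limit is measured on the absolute server clock, with no start time recorded.
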(event EventBeginPlay
  (Variables|Default|SetDurationGame (Math|Timespan|GetTotalSeconds (Math|Timespan|MakeTimespan 0 0 2))))

(event EventTick
  (params (DeltaSeconds :type Float%20%28single-precision%29))
  (if (and (> (GameState|GetServerWorldTimeSeconds) (Variables|Default|GetDurationGame)) (not (Variables|Default|GetJeuFini)))
    (Default|CallFinDuJeuDispatcher)
    (Variables|Default|SetJeuFini true)))

(fn ConstructionScript)