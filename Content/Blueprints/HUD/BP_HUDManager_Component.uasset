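; BP_HUDManager_Component manages the game's HUD widgets, swapping from the in-game HUD to an end-of-game screen.
; On BeginPlay it binds to the BP_TyranGameState end-of-game dispatcher, then creates and shows the HUD manager widget, stored as the timer widget.
; When the dispatcher fires, it removes that widget and displays BP_HUDFinDuJeu.
; A separate function creates and shows the guard-addition widget (BP_HUDAjoutGuarde).
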(event Custom|FinDuJeu
  (bind _returnvalue (UserInterface|CreateWidget "/Game/Blueprints/HUD/BP_HUDFinDuJeu.BP_HUDFinDuJeu_C"))
  (Widget|RemovefromParent (Variables|Default|GetWidget_Timer))
  (bind _output_get (Variables|Default|SetWidget_FinDuJeu _returnvalue))
  (UserInterface|Viewport|AddtoViewport _output_get 0))

(event EventTick
  (params (DeltaSeconds :type Float%20%28single-precision%29)))

(event EventBeginPlay
  (bind _asbp_tyran_game_state (Utilities|Casting|CastToBP_TyranGameState (Game|GetGameState)))
  (EventDispatchers|BindEventtoFinDuJeuDispatcher _asbp_tyran_game_state (delegate Custom|FinDuJeu))
  (bind _returnvalue (UserInterface|CreateWidget "/Game/Blueprints/HUD/BP_HUDManagerWidget.BP_HUDManagerWidget_C"))
  (bind _output_get (Variables|Default|SetWidget_Timer _returnvalue))
  (UserInterface|Viewport|AddtoViewport _output_get 0))

(fn CreateWidgetAjoutGuardes
  (bind _returnvalue (UserInterface|CreateWidget "/Game/Blueprints/HUD/BP_HUDAjoutGuarde.BP_HUDAjoutGuarde_C"))
  (bind _output_get (Variables|Default|SetWidget_AjoutGuarde _returnvalue))
  (UserInterface|Viewport|AddtoViewport _output_get 0))